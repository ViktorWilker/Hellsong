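; Player character Abdiel, with jump, dodge, interaction and switchable weapon move sets.
; On BeginPlay it hands itself to BPI_CharacterReferences actors; interaction uses a sphere trace, and move set changes are forwarded to the controller.
; Dodge compares movement input to actor axes via dot products, picking one of four montages, backward without input, when no montage is playing.
; Jumping re-enables shortly after landing; TryMove is a stub returning false.
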(event Input|EnhancedActionEvents|EnhancedInputActionIA_Interact
  (params (ActionValue :type Boolean) (ElapsedSeconds :type Float%20%28double-precision%29) (TriggeredSeconds :type Float%20%28double-precision%29) (InputAction :type Input%20Action%20Object%20Reference :default "/Game/ThirdPerson/Input/Actions/IA_Interact.IA_Interact"))
  (bind _returnvalue (Transformation|GetActorLocation))
  (:Triggered
    (bind (_outhit _returnvalue_2) (Collision|SphereTraceForObjects _returnvalue _returnvalue 1e+02 (Utilities|Array|MakeArray "ObjectTypeQuery7") false 0 "ForOneFrame"))
    (if _returnvalue_2
      (Class|BPIInteractable|Interact(Message) (.HitActor (Collision|BreakHitResult _outhit)) self))))

(event Input|EnhancedActionEvents|EnhancedInputActionIA_Jump
  (params (ActionValue :type Boolean) (ElapsedSeconds :type Float%20%28double-precision%29) (TriggeredSeconds :type Float%20%28double-precision%29) (InputAction :type Input%20Action%20Object%20Reference :default "/Game/ThirdPerson/Input/Actions/IA_Jump.IA_Jump"))
  (:Triggered
    (if (not (Variables|Default|GetIsJump))
      (Character|Jump)))
  (:Canceled
    (Character|StopJumping :!label _label))
  (:Completed
    (goto _label)))

(event EventBeginPlay
  (bind _outactors (Actor|GetAllActorswithInterface "/Game/Main/Interfaces/BPI_CharacterReferences.BPI_CharacterReferences_C"))
  (Class|BPICharacterReferences|Abdiel(Message) _outactors self))

(event EventSetMoveSet
  (params (Equipped :type Boolean) (MoveType :type Enum_MoveSets%20Enum :default "NewEnumerator2"))
  (Variables|Default|SetWeaponEquiped Equipped)
  (Variables|Default|SetCurrentMoveSet MoveType)
  (Class|BPICombatInterface|SwitchMoves(Message) (Pawn|GetController) MoveType))

(event EventOnJumped
  (Variables|Default|SetIsJump true))

(event EventOnLanded
  (params (Hit :type Hit%20Result%20Structure%20%28by%20ref%29))
  (Utilities|FlowControl|Delay 0.6)
  (Variables|Default|SetIsJump false))

(event Input|MouseEvents|ThumbMouseButton
  (params (Key :type Key%20Structure :default "None"))
  (:Pressed
    (if (CallFunction|IsIdle)
      (CallFunction|CalculateDesiredRotation)
      (CallFunction|SetDodgeAnimation)
      (Animation|PlayAnimMontage (Variables|Default|GetDodgeMontage) 1.0 "None"))))

(fn ConstructionScript)

(fn IsIdle
  (return (not (Animation|Montage|MontageIsPlaying (Components|SkeletalMesh|GetAnimInstance (Variables|Character|GetMesh)) 0))))

(fn IsEquipped
  (return (Variables|Default|GetWeaponEquiped)))

(fn GetMoveSet
  (return (Variables|Default|GetCurrentMoveSet)))

(fn CalculateDesiredRotation
  (bind (_dotforward _dotright) (CallFunction|ActorDotDirection))
  (bind (_dotforward_2 _dotright_2) (CallFunction|ActorDotDirection))
  (bind (_dotforward_3 _dotright_3) (CallFunction|ActorDotDirection))
  (bind (_dotforward_4 _dotright_4) (CallFunction|ActorDotDirection))
  (if (Utilities|Operators|NotEqual(!=) :A (Pawn|Components|PawnMovement|GetLastInputVector (Variables|Character|GetCharacterMovement)) :ErrorTolerance 0.0001)
    (if (and (> _dotforward_4 0.7) (and (>= _dotright_4 -0.7) (<= _dotright_4 0.7)))
      (Variables|Default|SetDesiredRotation "NewEnumerator2")
      (elif (and (< _dotforward_3 -0.7) (and (>= _dotright_3 -0.7) (<= _dotright_3 0.7)))
        (Variables|Default|SetDesiredRotation "NewEnumerator0")
        (elif (and (> _dotright_2 0.7) (and (>= _dotforward_2 -0.7) (<= _dotforward_2 0.7)))
          (Variables|Default|SetDesiredRotation "NewEnumerator1")
          (elif (and (< _dotright -0.7) (and (>= _dotforward -0.7) (<= _dotforward 0.7)))
            (Variables|Default|SetDesiredRotation "NewEnumerator3")))))
    (else
      (Variables|Default|SetDesiredRotation "NewEnumerator0"))))

(fn ActorDotDirection
  (bind _returnvalue (Class|Pawn|GetLastMovementInputVector))
  (bind _returnvalue_2 (Math|Vector|Normalize _returnvalue))
  (return (Math|Vector|DotProduct _returnvalue_2 (Transformation|GetActorForwardVector)) (Math|Vector|DotProduct _returnvalue_2 (Transformation|GetActorRightVector))))

(fn SetDodgeAnimation
  (switch Utilities|FlowControl|Switch|SwitchonEnum_DodgeDirction (Variables|Default|GetDesiredRotation)
    (:NewEnumerator2
      (Variables|Default|SetDodgeMontage "/Game/AnimationAssets/LigthSword_Moveset/LigthMovs/Dodge/DodgeF_Montage.DodgeF_Montage"))
    (:NewEnumerator0
      (Variables|Default|SetDodgeMontage "/Game/AnimationAssets/LigthSword_Moveset/LigthMovs/Dodge/DodgeB_Montage.DodgeB_Montage"))
    (:NewEnumerator1
      (Variables|Default|SetDodgeMontage "/Game/AnimationAssets/LigthSword_Moveset/LigthMovs/Dodge/DodgeR_Montage.DodgeR_Montage"))
    (:NewEnumerator3
      (Variables|Default|SetDodgeMontage "/Game/AnimationAssets/LigthSword_Moveset/LigthMovs/Dodge/DodgeL_Montage.DodgeL_Montage"))
    (:NewEnumerator4
      (Variables|Default|SetDodgeMontage "/Game/SwordAnimationPack/Animations/Dodge/DodgeF_Montage.DodgeF_Montage" :!label _label))
    (:NewEnumerator5
      (goto _label))
    (:NewEnumerator6
      (Variables|Default|SetDodgeMontage "/Game/SwordAnimationPack/Animations/Dodge/DodgeB_Montage.DodgeB_Montage" :!label _label_2))
    (:NewEnumerator7
      (goto _label_2))))

(fn TryMove
  (params (Command :type Input%20Command%20Object%20Reference) (Montage :type Anim%20Montage%20Object%20Reference))
  (return false))