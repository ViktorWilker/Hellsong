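; Base enemy character Blueprint for melee-style combat that can be targeted, deals hit damage and reacts to being hit.
; CollisionComponent uses the static mesh for hit detection and applies fixed point damage to actors that can receive it.
; Incoming damage feeds StatsComponent, then a standard-hit or knockdown montage plays based on player controller 0's current attack info, whoever the damage causer.
; Remaining query functions return fixed defaults, and TryMove always returns false.
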(event OnHit(CollisionComponent)
  (params (HitResult :type Hit%20Result%20Structure))
  (bind _returnvalue (Class|BPICombatInterface|CanRecieveDamage(Message) (.HitActor (Collision|BreakHitResult HitResult))))
  (if _returnvalue
    (Game|Damage|ApplyPointDamage 0 1e+01 (Transformation|GetActorForwardVector) HitResult (Game|GetInstigatorController) self)))

(event EventBeginPlay
  (Default|SetCollisionMeshComponent (Variables|Default|GetCollisionComponent) (Variables|Default|GetStaticMesh))
  (Default|AddActorstoIgnore (Variables|Default|GetCollisionComponent) self)
  (Class|StatsComponent|InitializeStats (Variables|Default|GetStatsComponent)))

(event Game|Damage|EventPointDamage
  (params (Damage :type Float%20%28single-precision%29) (DamageType :type Damage%20Type%20Object%20Reference) (HitLocation :type Vector :default "0, 0, 0") (HitNormal :type Vector :default "0, 0, 0") (HitComponent :type Primitive%20Component%20Object%20Reference) (BoneName :type Name :default "None") (ShotFromDirection :type Vector :default "0, 0, 0") (InstigatedBy :type Controller%20Object%20Reference) (DamageCauser :type Actor%20Object%20Reference) (HitInfo :type Hit%20Result%20Structure%20%28by%20ref%29))
  (Class|StatsComponent|TakeDamage (Variables|Default|GetStatsComponent) Damage)
  (bind _react (Class|BPICombatInterface|GetCurrentAttackInfos(Message) (Game|GetPlayerController 0)))
  (switch Utilities|FlowControl|Switch|SwitchonEnum_DamageReaction _react
    (:NewEnumerator0
      (Animation|PlayAnimMontage "/Game/AnimationAssets/Disarm_MoveSet/HitReaction/GhostSamurai_APose_Hit_F_Root_Montage_Enemy.GhostSamurai_APose_Hit_F_Root_Montage_Enemy" 1.0 "None"))
    (:NewEnumerator1
      (Animation|PlayAnimMontage "/Game/SwordAnimationPack/Animations/Roll/RollB_Montage.RollB_Montage" 1.0 "None"))))

(fn ConstructionScript)

(fn CanbeTarget
  (return true))

(fn CanRecieveDamage
  (return true))

(fn GetCurrentAttackInfos
  (return "NewEnumerator0" "NewEnumerator0"))

(fn GetMovementSpeedMode
  (return "NewEnumerator2"))

(fn TryMove
  (params (Command :type Input%20Command%20Object%20Reference) (Montage :type Anim%20Montage%20Object%20Reference))
  (return false))