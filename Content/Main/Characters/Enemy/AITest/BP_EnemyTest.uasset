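; BP_EnemyTest is a test katana-wielding enemy character with a patrol route and walk, jog and sprint speed modes.
; On BeginPlay it spawns a BP_EnemyWeapon attached to the sheath socket.
; Draw and disarm montages use notifies to move the sword between hand and sheath sockets and set the equipped flag.
; Attack, draw and disarm each fire an end dispatcher on completion or interruption.
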(event Custom|Attack
  (Animation|Montage|PlayMontage (Variables|Character|GetMesh) "/Game/SwordAnimationPack/Animations/Attacks/Attack1_Montage.Attack1_Montage"
    (:OnCompleted
      _)
    (:OnInterrupted
      _))
  (Default|CallOnAttackEnd))

(event Custom|WieldSword
  (bind _notifyname (Animation|Montage|PlayMontage (Variables|Character|GetMesh) "/Game/AnimationAssets/LigthSword_Moveset/EnemyDraw.EnemyDraw")
    (:OnCompleted
      (Default|CallOnEquiped :!label _label))
    (:OnInterrupted
      (goto _label))
    (:OnNotifyBegin
      (switch name _notifyname
        (:Hold
          (Transformation|AttachComponentToComponent (Variables|Default|GetSword) (Variables|Character|GetMesh) "KatanaHand" "SnapToTarget" "SnapToTarget" "SnapToTarget" true)
          (Variables|Default|SetEquipSword true))))))

(event Custom|SpawnSword
  (bind _self self)
  (bind _returnvalue (Game|SpawnActorfromClass "/Game/Main/Characters/Enemy/AITest/BP_EnemyWeapon.BP_EnemyWeapon_C" (Transformation|GetActorTransform) "Undefined" "MultiplyWithRoot" _self _self))
  (bind _output_get (Variables|Default|SetSword _returnvalue))
  (Transformation|AttachComponentToComponent _output_get (Variables|Character|GetMesh) "KatanaSheath" "SnapToTarget" "SnapToTarget" "SnapToTarget" true))

(event Custom|DisarmSword
  (bind _notifyname (Animation|Montage|PlayMontage (Variables|Character|GetMesh) "/Game/AnimationAssets/LigthSword_Moveset/EnemyDisarm.EnemyDisarm")
    (:OnCompleted
      (Default|CallOnDisarm :!label _label))
    (:OnInterrupted
      (goto _label))
    (:OnNotifyBegin
      (switch name _notifyname
        (:Disarm
          (Transformation|AttachComponentToComponent (Variables|Default|GetSword) (Variables|Character|GetMesh) "KatanaSheath" "SnapToTarget" "SnapToTarget" "SnapToTarget" true)
          (Variables|Default|SetEquipSword false))))))

(event EventBeginPlay
  (CallFunction|SpawnSword))

(fn ConstructionScript)

(fn GetPatrolRoute
  (return (Variables|IA|GetPatrolPath)))

(fn SetMovementSpeedMode
  (params (Movement :type Enum_MovementSpeedMode%20Enum :default "NewEnumerator2"))
  (bind _output_get (Variables|/Script/Engine.CharacterMovementComponent|SetMaxWalkSpeed (Variables|Character|GetCharacterMovement) (Utilities|Select :Index Movement :NewEnumerator2 2e+02 :NewEnumerator0 4e+02 :NewEnumerator1 6e+02)))
  (return _output_get))