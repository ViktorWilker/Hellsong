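; BP_BaseEnemy_Child is an enemy character Blueprint, apparently derived from a base enemy, that handles incoming point damage.
; On point damage it passes the amount to its StatsComponent, sets HitFront from a FrontHit check on the instigator, then calls HitReaction.
; BeginPlay, overlap and Tick are disabled placeholder nodes, and the construction script only calls the parent.
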(event EventBeginPlay
  (|CallParentFunction) ; This node is disabled and will not be called.\nDrag off pins to build functionality.
)

(event Collision|EventActorBeginOverlap
  (params (OtherActor :type Actor%20Object%20Reference))
  (|CallParentFunction OtherActor) ; This node is disabled and will not be called.\nDrag off pins to build functionality.
)

(event EventTick
  (params (DeltaSeconds :type Float%20%28single-precision%29))
  (|CallParentFunction DeltaSeconds) ; This node is disabled and will not be called.\nDrag off pins to build functionality.
)

(event Game|Damage|EventPointDamage
  (params (Damage :type Float%20%28single-precision%29) (DamageType :type Damage%20Type%20Object%20Reference) (HitLocation :type Vector :default "0, 0, 0") (HitNormal :type Vector :default "0, 0, 0") (HitComponent :type Primitive%20Component%20Object%20Reference) (BoneName :type Name :default "None") (ShotFromDirection :type Vector :default "0, 0, 0") (InstigatedBy :type Controller%20Object%20Reference) (DamageCauser :type Actor%20Object%20Reference) (HitInfo :type Hit%20Result%20Structure%20%28by%20ref%29))
  (Class|StatsComponent|TakeDamage (Variables|Default|GetStatsComponent) Damage)
  (Variables|Default|SetHitFront (CallFunction|FrontHit InstigatedBy))
  (CallFunction|HitReaction))

(fn ConstructionScript
  (|CallParentFunction))