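; Player controller for combat that possesses BP_Abdiel, registers with the game instance and creates the in-game HUD widget.
; When buffered input arrives and the character is idle, it matches the buffer against parallel command and montage arrays, plays the matching montage and clears the history.
; Helpers load moves from a combat data table, check state tags, detect dodge input and track action priority, alongside several stubbed getters.
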(event Custom|ResolveBuffer
  (bind (_array_element _array_index) (Utilities|Array|ForEachLoopwithBreak (Variables|Default|GetCommands))
    (:LoopBody
      (bind _success (CallFunction|TryMove _array_element (Utilities|Array|Get(acopy) (Variables|Default|GetMontages) _array_index)))
      (if _success
        (CallFunction|BreakMoves)))))

(event Custom|BreakMoves
  (Utilities|Array|ForEachLoopwithBreak (Variables|Default|GetCommands)) ; enters at Break
)

(event EventPossess
  (params (PossessedPawn :type Pawn%20Object%20Reference))
  (|CallParentFunction PossessedPawn)
  (bind _asbp_abdiel (Utilities|Casting|CastToBP_Abdiel PossessedPawn))
  (Variables|Default|SetCharacterReference _asbp_abdiel))

(event EventPostBufferInput
  (bind _characterreference (Variables|Default|GetCharacterReference))
  (Development|PrintString (Class|InputBufferComponent|Print (Variables|Default|GetInputBuffer) 0 false false))
  (Utilities|IsValid _characterreference
    (:Is%20Valid
      (if (Default|IsIdle _characterreference)
        (CallFunction|ResolveBuffer)))))

(event EventBeginPlay
  (Class|BPICharacterReferences|SetCombatController(Message) (Game|GetGameInstance) self)
  (bind _returnvalue (UserInterface|CreateWidget "/Game/Main/UI/Widgets/W_InGame.W_InGame_C" self))
  (bind _output_get (Variables|Default|SetW_InGame _returnvalue))
  (UserInterface|Viewport|AddtoViewport _output_get 0))

(fn ConstructionScript)

(fn SetInitialMoves
  (bind _outrownames (DataTable|GetDataTableRowNames (Variables|Default|GetCurrentCombatData)))
  (for _array_element _outrownames
    (bind _returnvalue (Utilities|GetDataTableRow (Variables|Default|GetCurrentCombatData) _array_element)
      (:then
        (bind _returnvalue_2 (Utilities|Array|Add (Variables|Default|GetActionData) (Utilities|Struct|MakeS_CharacterMoveSet (.ActionID (Utilities|Struct|BreakS_CharacterMoveSet _returnvalue)) "(TagName=\"\")" 0 false "(TagName=\"\")" false false (.Command (Utilities|Struct|BreakS_CharacterMoveSet _returnvalue)) (.Montage (Utilities|Struct|BreakS_CharacterMoveSet _returnvalue)) (.NextActionID (Utilities|Struct|BreakS_CharacterMoveSet _returnvalue)))))
        (Development|PrintString (Utilities|String|ToString(Integer) _returnvalue_2))))))

(fn ClearMoves
  (Utilities|Array|Clear (Variables|Default|GetMontages))
  (Utilities|Array|Clear (Variables|Default|GetCommands)))

(fn SetCombatData
  (params (CurrentCombatData :type Data%20Table%20Object%20Reference))
  (Variables|Default|SetCurrentCombatData CurrentCombatData))

(fn GetCombatData
  (return (Variables|Default|GetCurrentCombatData)))

(fn DodgeAttack
  (Default|CalculateDesiredRotation (CallFunction|GetCombatPlayer)))

(fn IsDodgeEvent
  (return (Utilities|Array|ContainsItem (Class|InputBufferComponent|GetCurrentEvents (Variables|Default|GetInputBuffer)) "dodge")))

(fn CheckBestPriority
  (params (Priority :type Integer) (Action :type S%20Character%20Move%20Set%20Structure))
  (if (> Priority (Variables|Default|GetGreaterPriority))
    (Variables|Default|SetGreaterPriority Priority :!label _label)
    (Variables|Default|SetCurrentAction Action)
    (return)
    (elif (and (== Priority (Variables|Default|GetGreaterPriority)) (== (.ActionID (Utilities|Struct|BreakS_CharacterMoveSet Action)) ""))
      (goto _label))))

(fn CheckCurrentState
  (params (GameplayTagContainer :type Gameplay%20Tag%20Container%20Structure%20%28by%20ref%29))
  (bind _gameplaytags (GameplayTags|BreakGameplayTagContainer GameplayTagContainer))
  (bind _returnvalue (CallFunction|GetCombatPlayer))
  (bind _statemanager (Variables|/Script/Hellsong.HMainCharacter|GetStateManager _returnvalue))
  (bind _returnvalue_2 (Class|StateManagerComponent|GetCurrentState _statemanager))
  (if (or (== (GameplayTags|GetTagName (Utilities|Array|Get(acopy) _gameplaytags)) _returnvalue_2) (== (GameplayTags|GetTagName (Utilities|Array|Get(acopy) _gameplaytags 1)) _returnvalue_2))
    (return true)
    (else
      (return false))))

(fn GetDatatableRowbyCommand
  (bind _outrownames (DataTable|GetDataTableRowNames "/Game/Main/DataStrcuts/DT_Katana_MoveSet.DT_Katana_MoveSet"))
  (for _array_element _outrownames
    (bind _returnvalue (Utilities|GetDataTableRow "/Game/Main/DataStrcuts/DT_Katana_MoveSet.DT_Katana_MoveSet" _array_element)
      (:then
        (Development|PrintString (Utilities|GetDisplayName (.Command (Utilities|Struct|BreakS_CharacterMoveSet _returnvalue))))))))

(fn CanRecieveDamage
  (return false))

(fn GetCombatController
  (return 0))

(fn GetCurrentAttackInfos
  (return (Variables|Default|GetDamage%20Type) (Variables|Default|GetDamage%20Reaction)))

(fn GetMovementSpeedMode
  (return "NewEnumerator2"))

(fn GetPlayer
  (return 0))

(fn TryMove
  (params (Command :type Input%20Command%20Object%20Reference) (Montage :type Anim%20Montage%20Object%20Reference))
  (bind _output_get (LocalVariables|SetSuscess (Class|InputBufferComponent|MatchCommand (Variables|Default|GetInputBuffer) Command)))
  (if _output_get
    (Animation|PlayAnimMontage (Variables|Default|GetCharacterReference) Montage 1.0 "None")
    (Class|InputBufferComponent|ClearHistory (Variables|Default|GetInputBuffer))
    (return (LocalVariables|GetSuscess))
    (else
      (return (LocalVariables|GetSuscess)))))