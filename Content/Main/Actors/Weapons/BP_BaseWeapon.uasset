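; Base weapon Blueprint that connects an equipped item to its owner's combat component and move set.
; The construction script scans DT_WeaponsSetup for the row matching MoveSet, copying its hand and sheathed sockets and combat enter/exit settings.
; On equip, it registers as the CombatComponent's main weapon and passes the item mesh to its collision component.
; Changing hand attachment broadcasts a move-set update through the GameInstance's player message object.
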(event EventBeginPlay
  (|CallParentFunction) ; This node is disabled and will not be called.\nDrag off pins to build functionality.
)

(event Collision|EventActorBeginOverlap
  (params (OtherActor :type Actor%20Object%20Reference))
  (|CallParentFunction OtherActor) ; This node is disabled and will not be called.\nDrag off pins to build functionality.
)

(event EventTick
  (params (DeltaSeconds :type Float%20%28single-precision%29))
  (|CallParentFunction DeltaSeconds) ; This node is disabled and will not be called.\nDrag off pins to build functionality.
)

(event EventOnEquipped
  (|CallParentFunction)
  (bind _output_get (Variables|Default|SetCombatComponent (Actor|GetComponentbyClass (Components|GetOwner) "/Game/Main/Components/CombatComponent.CombatComponent_C")))
  (Default|SetMainWeapon _output_get self)
  (Utilities|IsValid _output_get
    (:Is%20Valid
      (Default|SetCollisionMeshComponent (Variables|Default|GetCollisionComponent) (Class|HBaseEquippable|GetItemMesh)))))

(fn ConstructionScript
  (|CallParentFunction)
  (bind _outrownames (DataTable|GetDataTableRowNames "/Game/Main/DataStrcuts/DT_WeaponsSetup.DT_WeaponsSetup"))
  (for _array_element _outrownames
    (bind _returnvalue (Utilities|GetDataTableRow "/Game/Main/DataStrcuts/DT_WeaponsSetup.DT_WeaponsSetup" _array_element)
      (:then
        (if (Utilities|Enum|Equal(Enum) (.WeaponID (Utilities|Struct|BreakS_WeaponSetup _returnvalue)) (Variables|Config|GetMoveSet))
          (Variables|Attachment|SetHandEquipSocket (.HandSocket (Utilities|Struct|BreakS_WeaponSetup _returnvalue)))
          (Variables|Default|SetEquipedSocket (.SheathedSocket (Utilities|Struct|BreakS_WeaponSetup _returnvalue)))
          (Variables|CombatAnims|SetEnterCombat (.EnterCombat (Utilities|Struct|BreakS_WeaponSetup _returnvalue)))
          (Variables|CombatAnims|SetExitCombat (.ExitCombat (Utilities|Struct|BreakS_WeaponSetup _returnvalue))))))))

(fn SetAttachedtoHand
  (params (bIsAttachedToHand :type Boolean))
  (bind _output_get (Variables|Attachment|SetbIsAttachedToHand bIsAttachedToHand))
  (bind _returnvalue (Class|BPICharacterReferences|GetPlayer(Message) (Game|GetGameInstance)))
  (if _output_get
    (Class|BPICombatInterface|UpdateMoveSet(Message) _returnvalue true (Variables|Config|GetMoveSet))
    (else
      (Class|BPICombatInterface|UpdateMoveSet(Message) _returnvalue false "NewEnumerator2"))))

(fn IsAttachedtoHand
  (return (Variables|Attachment|GetbIsAttachedToHand)))